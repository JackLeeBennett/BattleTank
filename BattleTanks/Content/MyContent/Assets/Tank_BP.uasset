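; Tank Blueprint that handles orbit-style camera aiming for a tank.
; On BeginPlay it passes its Barrel component to SetBarrelReferance.
; The AimAzimuth axis yaws the AzimuthGimble and AimElevation pitches the SpringArm, keeping the two rotations on separate components.
; Both inputs apply local rotation scaled by world delta seconds for frame-rate-independent movement.
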(event `self.ReceiveBeginPlay`
  (`self.SetBarrelReferance` (`self.Barrel`)))

(event `InputAxis|AimAzimuth`
  (params (AxisValue :type "Float (single-precision)"))
  ;[1 1 1] Camera input binding
  (`SceneComponent.K2_AddLocalRotation` (`self.Azimuth Gimble`) (`KismetMathLibrary.MakeRotator` 0.0 0.0 (* AxisValue (`GameplayStatics.GetWorldDeltaSeconds`) 100.0)) false false))

(event `InputAxis|AimElevation`
  (params (AxisValue :type "Float (single-precision)"))
  ;[1 1 1] Camera input binding
  (`SceneComponent.K2_AddLocalRotation` (`self.SpringArm`) (`KismetMathLibrary.MakeRotator` 0.0 (* AxisValue (`GameplayStatics.GetWorldDeltaSeconds`) 100.0)) false false))

(fn `UserConstructionScript`)